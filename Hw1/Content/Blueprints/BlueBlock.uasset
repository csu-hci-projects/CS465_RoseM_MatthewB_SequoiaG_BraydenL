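; BlueBlock is a cube actor that changes color while a ControllerColider actor overlaps it.
; The construction script creates a dynamic material instance from CubeColor, sets it to Color1 and applies it to the Cube.
; Begin and end overlap events switch the material's Color parameter to Color2 and back to Color1, ignoring other actor types.
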(event `self.ReceiveActorBeginOverlap`
  (params (OtherActor :type "Actor Object Reference"))
  (cast `/Game/Blueprints/ControllerColider` OtherActor)
  (`MaterialInstanceDynamic.SetVectorParameterValue` (`self.Material`) "Color" (`KismetMathLibrary.Conv_ColorToLinearColor` (`self.Color2`))))

(event `self.ReceiveActorEndOverlap`
  (params (OtherActor :type "Actor Object Reference"))
  (cast `/Game/Blueprints/ControllerColider` OtherActor)
  (`MaterialInstanceDynamic.SetVectorParameterValue` (`self.Material`) "Color" (`KismetMathLibrary.Conv_ColorToLinearColor` (`self.Color1`))))

(fn `UserConstructionScript`
  ;[1 1 1] Create Dynamic Mateiral
  (bind _returnvalue (`KismetMaterialLibrary.CreateDynamicMaterialInstance` "/Game/Materials/CubeColor.CubeColor"))
  (bind _output_get (set `self.Material` _returnvalue))
  (`MaterialInstanceDynamic.SetVectorParameterValue` _output_get "Color" (`KismetMathLibrary.Conv_ColorToLinearColor` (`self.Color1`)))
  (`PrimitiveComponent.SetMaterial` (`self.Cube`) 0 (`self.Material`)))